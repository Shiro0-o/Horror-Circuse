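; BP_Birck_Wall procedurally builds a wall, presumably of bricks, in its Construction Script.
; Each mesh in the StaticMesh array gets its own Hierarchical Instanced Static Mesh component, collected in HISMArrayRef.
; A Y-Z grid, sized and spaced by count and offset variables, places each instance on a randomly picked component.
; The grid loop runs inside the mesh loop, so every mesh adds another full grid at the same positions.
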(event EventBeginPlay)

(event Collision|EventActorBeginOverlap
  (params (OtherActor :type Actor%20Object%20Reference)))

(event EventTick
  (params (DeltaSeconds :type Float%20%28single-precision%29)))

(fn ConstructionScript
  (Components|InstancedStaticMesh|ClearInstances (Variables|Default|GetHISM%20Ref))
  (for _array_element (Variables|Default|GetStatic%20Mesh%20)
    (bind _output_get (Variables|Default|SetMesh%20Ref _array_element))
    (bind _returnvalue (AddComponent|AddHierarchicalInstancedStaticMeshComponent false))
    (bind _output_get_2 (Variables|Default|SetHISM%20Ref _returnvalue))
    (Utilities|Array|AddUnique (Variables|Default|GetHISM%20Array%20Ref) _output_get_2)
    (Components|StaticMesh|SetStaticMesh _output_get_2 _output_get)
    (for _index (range 0 (- (Variables|Default|GetX%20Offset) 1))
      (Variables|Default|SetX%20Location (Math|Vector|MakeVector 0.0 (.x (* _index (Variables|Default|GetOffset%20Y))) 0.0))
      (for _index_2 (range 0 (- (Variables|Default|GetZ%20Offset) 1))
        (Variables|Default|SetZ%20Location (Math|Vector|MakeVector 0.0 0.0 (+ (.z (* _index_2 (Variables|Default|GetOffset%20Z))) (Variables|Default|GetMesh_Offset))))
        (Components|InstancedStaticMesh|AddInstance (.OutItem (Utilities|Array|Random (Variables|Default|GetHISM%20Array%20Ref))) (Math|Transform|MakeTransform (+ (Variables|Default|GetX%20Location) (Variables|Default|GetZ%20Location)) "0.0,0.0,0.0" "1.000000,1.000000,1.000000") false)))))