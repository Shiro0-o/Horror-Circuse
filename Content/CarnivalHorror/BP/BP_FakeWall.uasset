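; BP_FakeWall is a spline-driven fake wall, built in the construction script with no active runtime logic.
; It divides the spline length by Offset and adds a spline mesh component for each step, shaped between consecutive distances in local space.
; Segment tangents are normalized spline tangents scaled by length divided by Offset, the segment count, rather than by segment length.
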(event EventBeginPlay)

(event Collision|EventActorBeginOverlap
  (params (OtherActor :type Actor%20Object%20Reference)))

(event EventTick
  (params (DeltaSeconds :type Float%20%28single-precision%29)))

(fn ConstructionScript
  (bind _spline (Variables|Default|GetSpline))
  (bind _offset (Variables|Default|GetOffset))
  (bind _returnvalue (Spline|GetSplineLength _spline))
  (bind _returnvalue_2 (/ _returnvalue _offset))
  (for _index (range 0 (Math|Float|Truncate (/ _returnvalue _offset)))
    (bind _returnvalue_3 (AddComponent|AddSplineMeshComponent false))
    (SplineMesh|SetStartandEnd _returnvalue_3 (Spline|GetLocationatDistanceAlongSpline (Variables|Default|GetSpline) (* _index _offset) "Local") (* (Math|Vector|Normalize (Spline|GetTangentatDistanceAlongSpline (Variables|Default|GetSpline) (* _index _offset) "Local")) _returnvalue_2) (Spline|GetLocationatDistanceAlongSpline (Variables|Default|GetSpline) (* (+ _index 1) _offset) "Local") (* (Math|Vector|Normalize (Spline|GetTangentatDistanceAlongSpline (Variables|Default|GetSpline) (* (+ _index 1) _offset) "Local")) _returnvalue_2) true :!class /Script/Engine.SplineMeshComponent)))