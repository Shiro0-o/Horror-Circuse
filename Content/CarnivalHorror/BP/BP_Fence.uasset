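; BP_Fence is a construction-time tool that lays out a fence along an editable spline.
; The construction script places SMFence instances through a HISM component at every Offset distance, without setting their rotation.
; A second loop adds a spline mesh component between consecutive points, using normalized spline tangents scaled by spline length divided by Offset.
; The event graph has no active logic.
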(event EventBeginPlay)

(event Collision|EventActorBeginOverlap
  (params (OtherActor :type Actor%20Object%20Reference)))

(event EventTick
  (params (DeltaSeconds :type Float%20%28single-precision%29)))

(fn ConstructionScript
  (bind _spline (Variables|Default|GetSpline))
  (bind _offset (Variables|Default|GetOffset))
  (bind _returnvalue (Spline|GetSplineLength _spline))
  (bind _returnvalue_2 (/ _returnvalue _offset))
  (bind _returnvalue_3 (/ _returnvalue _offset))
  (bind _returnvalue_4 (Math|Float|Truncate _returnvalue_2))
  (Components|StaticMesh|SetStaticMesh (Variables|Default|GetHISM) (Variables|Default|GetSM_Fence))
  (for _index (range 0 _returnvalue_4)
    (Components|InstancedStaticMesh|AddInstance (Variables|Default|GetHISM) (Math|Transform|MakeTransform (Spline|GetLocationatDistanceAlongSpline (Variables|Default|GetSpline) (* _index _offset) "Local") "0, 0, 0" "1.000000,1.000000,1.000000") false))
  (for _index_2 (range 0 _returnvalue_4)
    (bind _returnvalue_5 (AddComponent|AddSplineMeshComponent false))
    (SplineMesh|SetStartandEnd _returnvalue_5 (Spline|GetLocationatDistanceAlongSpline (Variables|Default|GetSpline) (* _index_2 _offset) "Local") (* (Math|Vector|Normalize (Spline|GetTangentatDistanceAlongSpline (Variables|Default|GetSpline) (* _index_2 _offset) "Local")) _returnvalue_3) (Spline|GetLocationatDistanceAlongSpline (Variables|Default|GetSpline) (* (+ _index_2 1) _offset) "Local") (* (Math|Vector|Normalize (Spline|GetTangentatDistanceAlongSpline (Variables|Default|GetSpline) (* (+ _index_2 1) _offset) "Local")) _returnvalue_3) true :!class /Script/Engine.SplineMeshComponent)))