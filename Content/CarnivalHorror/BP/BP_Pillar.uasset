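; BP_Pillar is a construction-time placement tool that builds a straight row of pillar meshes.
; The construction script assigns the chosen static mesh to an instanced mesh component (HISM), then adds the requested number of instances along local X at a fixed offset.
; Each instance gets a uniform scale and a random yaw from a random stream, so the variation is repeatable.
; The event graph holds no logic.
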(event EventBeginPlay)

(event Collision|EventActorBeginOverlap
  (params (OtherActor :type Actor%20Object%20Reference)))

(event EventTick
  (params (DeltaSeconds :type Float%20%28single-precision%29)))

(fn ConstructionScript
  (bind _static_mesh (Variables|Default|GetStatic%20Mesh))
  (bind _returnvalue (StaticMesh|GetBoundingBox _static_mesh))
  (Components|StaticMesh|SetStaticMesh (Variables|Default|GetHISM) (Variables|Default|GetStatic%20Mesh))
  (if (>= (Variables|Default|GetNb_Pillar) 0)
    (Variables|Default|SetBound_Mesh%20X (.x (- (.max _returnvalue) (.min _returnvalue))))
    (for _index (range 0 (- (Variables|Default|GetNb_Pillar) 1))
      (bind _output_get (Variables|Default|SetNew%20Location (Math|Vector|MakeVector (* _index (Variables|Default|GetOffset)) 0.0 0.0)))
      (Components|InstancedStaticMesh|AddInstance (Variables|Default|GetHISM) (Math|Transform|MakeTransform _output_get (Math|Rotator|MakeRotator 0.0 0.0 (Math|Random|RandomFloatinRangefromStream (Variables|Default|GetStream) 0.0 3.6e+02)) (Math|Conversions|ToVector(Float) (Variables|Default|GetScale))) false))))