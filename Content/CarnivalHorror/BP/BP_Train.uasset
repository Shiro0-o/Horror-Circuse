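; BP_Train is a train actor that moves its SMKidsTrain01 component along a referenced BP_Rail spline, starting at BeginPlay.
; A Timeline runs at a play rate of 1/Speed, so a higher Speed value gives a slower trip.
; Its alpha maps to distance along the spline, setting the component's relative location to the world point minus actor location and applying the world rotation as relative.
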(event Custom|MoveObject
  (Components|Timeline|SetPlayRate (Variables|Default|GetTimeline) (/ 1.0 (Variables|Default|GetSpeed)))
  (bind _alpha (Timeline|Timeline PlayFromStart)
    (:Update
      (Transformation|SetRelativeLocationAndRotation (Variables|Default|GetSM_KidsTrain01) (- (Spline|GetLocationatDistanceAlongSpline (Variables|/Game/CarnivalHorror/BP/BP_Rail.BP_Rail_C|GetSpline (stale EventBeginPlay _asbp_rail)) (Math|Float|Lerp 0.0 (Spline|GetSplineLength (Variables|/Game/CarnivalHorror/BP/BP_Rail.BP_Rail_C|GetSpline (stale EventBeginPlay _asbp_rail))) _alpha) "World") (Transformation|GetActorLocation)) (Spline|GetRotationatDistanceAlongSpline (Variables|/Game/CarnivalHorror/BP/BP_Rail.BP_Rail_C|GetSpline (stale EventBeginPlay _asbp_rail)) (Math|Float|Lerp 0.0 (Spline|GetSplineLength (Variables|/Game/CarnivalHorror/BP/BP_Rail.BP_Rail_C|GetSpline (stale EventBeginPlay _asbp_rail))) _alpha) "World") false false))))

(event EventBeginPlay
  (bind _asbp_rail (Utilities|Casting|CastToBP_Rail (Variables|Default|GetBP_Rail)))
  (CallFunction|MoveObject))

(fn ConstructionScript)