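; Procedural stone tower actor that builds stacked rings of mesh instances in the construction script.
; Each stage generates a circular spline with computed tangents, sizes the stone count from mesh bounds and radius, then places HISM instances with random radial offset and color custom data.
; On BeginPlay, Platon converts any components in StaticMeshCompArray into new HISMs and destroys the originals.
; The reposition and cleanup chains in EventGraph are unconnected.
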(event EventBeginPlay
  (CallFunction|Platon))

(fn ConstructionScript
  (bind _hism (Variables|Default|GetHISM))
  (bind _spline_cube_color (Variables|Default|GetSpline%20Cube%20Color))
  (bind (_r _g _b) (Utilities|Struct|BreakLinearColor _spline_cube_color))
  (bind _staticmesh (Variables|/Script/Engine.StaticMeshComponent|GetStaticMesh _hism))
  (bind _returnvalue (StaticMesh|GetBoundingBox _staticmesh))
  (Components|InstancedStaticMesh|ClearInstances (Variables|Default|GetHISM))
  (Components|StaticMesh|SetStaticMesh (Variables|Default|GetHISM) (Variables|Default|GetStatic%20Mesh))
  (Rendering|Material|SetMaterial (Variables|Default|GetHISM) 0 (Variables|Default|GetMaterial))
  (if (> (Variables|Default|GetNb%20Stage) 0)
    ;[1 1 1] Get Mesh Bound
    (for _index (range 0 (- (Variables|Default|GetNb%20Stage) 1))
      (Variables|Default|SetIndex%20Nb%20Stage _index)
      (Variables|Default|SetOffset%20Stone (- (.max _returnvalue) (.min _returnvalue)))
      (Variables|Default|SetZ%20Offset_Spline (/ (.z (Variables|Default|GetOffset%20Stone)) 2.0))
      (Variables|Default|SetRadius%20Offset (/ (.x (Variables|Default|GetOffset%20Stone)) -1.5))
      (bind _returnvalue_2 (AddComponent|AddSplineComponent false))
      (Variables|Default|SetL%20Spline%20Component _returnvalue_2)
      (Spline|ClearSplinePoints (Variables|Default|GetL%20Spline%20Component) true)
      (Variables|Default|SetStone_Cercle (- (Math|Float|Truncate (/ 3.6e+02 (* (Math|Trig|RadiansToDegrees (Class|KismetMathLibrary|Asin (/ (/ (.X (Math|Vector|BreakVector (Variables|Default|GetOffset%20Stone))) 2.0) (Variables|Default|GetL_Radius)))) 2.0))) 1))
      ;[1 1 1] Set Tangeant
      (for _index_2 (range 0 (- (Variables|Default|GetL_SplinePoints) 1))
        (Variables|Default|SetL_Index%20Point _index_2)
        (Variables|Default|SetL_SplinePoint (Math|Vector|MakeVector (* (Math|Trig|Sin(Degrees) (Math|Float|MapRangeClamped (Math|Conversions|ToFloat(Integer) (Variables|Default|GetL_Index%20Point)) 0.0 (Math|Conversions|ToFloat(Integer) (- (Variables|Default|GetL_SplinePoints) 1)) 0.0 (Math|Conversions|ToFloat(Integer) (|(360-(360/Segments)) (Variables|Default|GetL_SplinePoints))))) (Variables|Default|GetL_Radius)) (* (Math|Trig|Cos(Degrees) (Math|Float|MapRangeClamped (Math|Conversions|ToFloat(Integer) (Variables|Default|GetL_Index%20Point)) 0.0 (Math|Conversions|ToFloat(Integer) (- (Variables|Default|GetL_SplinePoints) 1)) 0.0 (Math|Conversions|ToFloat(Integer) (|(360-(360/Segments)) (Variables|Default|GetL_SplinePoints))))) (Variables|Default|GetL_Radius)) (+ (* (Variables|Default|GetIndex%20Nb%20Stage) (.z (Variables|Default|GetOffset%20Stone))) (Variables|Default|GetZ%20Offset_Spline))))
        (Spline|AddSplinePoint (Variables|Default|GetL%20Spline%20Component) (Variables|Default|GetL_SplinePoint) "Local" true)
        (Variables|Default|SetL_Rotation (Math|Rotator|FindLookatRotation (Variables|Default|GetL_SplinePoint) (Math|Vector|MakeVector 0.0 0.0 0.0)))
        (Variables|Default|SetL_TangentAtSplinePoint (* (Math|Vector|GetRightVector (Variables|Default|GetL_Rotation)) (* (Variables|Default|GetL_Radius) (|(4*(tan(((D2R((360/Segments)))/4)))) (Variables|Default|GetL_SplinePoints)))))
        (Spline|SetTangentatSplinePoint (Variables|Default|GetL%20Spline%20Component) (Variables|Default|GetL_Index%20Point) (Variables|Default|GetL_TangentAtSplinePoint) "Local" true))
      ;[1 1 1] Set Location at Mesh
      (for _index_3 (range 0 (- (Variables|Default|GetStone_Cercle) 2))
        (bind _output_get (Variables|Default|SetSton%20Index _index_3))
        (Variables|Default|SetL%20Stone%20SplineX (- (Spline|GetLocationatDistanceAlongSpline (Variables|Default|GetL%20Spline%20Component) (* _output_get (/ (Spline|GetSplineLength (Variables|Default|GetL%20Spline%20Component)) (Math|Conversions|ToFloat(Integer) (- (Variables|Default|GetStone_Cercle) 1)))) "Local") (* (Math|Vector|GetForwardVector (Math|Rotator|FindLookatRotation (Spline|GetLocationatDistanceAlongSpline (Variables|Default|GetL%20Spline%20Component) (* _output_get (/ (Spline|GetSplineLength (Variables|Default|GetL%20Spline%20Component)) (Math|Conversions|ToFloat(Integer) (- (Variables|Default|GetStone_Cercle) 1)))) "Local") (Math|Vector|MakeVector 0.0 0.0 (.Z (Math|Vector|BreakVector (Spline|GetLocationatDistanceAlongSpline (Variables|Default|GetL%20Spline%20Component) (* _output_get (/ (Spline|GetSplineLength (Variables|Default|GetL%20Spline%20Component)) (Math|Conversions|ToFloat(Integer) (- (Variables|Default|GetStone_Cercle) 1)))) "Local")))))) (+ (Variables|Default|GetRadius%20Offset) (Math|Random|RandomFloatinRange (Variables|Default|GetRadius%20Offset%20Min) (Variables|Default|GetRadius%20Offset%20Max))))))
        (Variables|Default|SetL%20Stone%20Spline%20Rotation (Spline|GetRotationatDistanceAlongSpline (Variables|Default|GetL%20Spline%20Component) (* _output_get (/ (Spline|GetSplineLength (Variables|Default|GetL%20Spline%20Component)) (Math|Conversions|ToFloat(Integer) (- (Variables|Default|GetStone_Cercle) 1)))) "Local"))
        ;[1 1 1] Add Instance And Mat
        (bind _returnvalue_3 (Components|InstancedStaticMesh|AddInstance (Variables|Default|GetHISM) (Math|Transform|MakeTransform (Variables|Default|GetL%20Stone%20SplineX) (Variables|Default|GetL%20Stone%20Spline%20Rotation) (Math|Conversions|ToVector(Float) (Variables|Default|GetStone%20Scale))) false))
        (Variables|Default|SetStone%20on%20Splin%20Index _returnvalue_3)
        (Components|InstancedStaticMesh|SetCustomDataValue (Variables|Default|GetHISM) (Variables|Default|GetStone%20on%20Splin%20Index) 0 _r false)
        (Components|InstancedStaticMesh|SetCustomDataValue (Variables|Default|GetHISM) (Variables|Default|GetStone%20on%20Splin%20Index) 1 _g false)
        (Components|InstancedStaticMesh|SetCustomDataValue (Variables|Default|GetHISM) (Variables|Default|GetStone%20on%20Splin%20Index) 2 _b false)))))

(fn Platon
  (bind _static_mesh_comp_array (Variables|Default|GetStatic%20Mesh%20Comp%20Array))
  (bind _static_mesh_comp_array_2 (Variables|Default|GetStatic%20Mesh%20Comp%20Array))
  (if (Utilities|Array|IsValidIndex _static_mesh_comp_array)
    (for _array_element _static_mesh_comp_array
      (LocalVariables|SetArray%20Element _array_element)
      (Rendering|SetVisibility (LocalVariables|GetArray%20Element) false false)
      (bind _returnvalue (AddComponent|AddHierarchicalInstancedStaticMeshComponent false))
      (bind _output_get (LocalVariables|SetHISM%20Ref _returnvalue))
      (Utilities|Array|AddUnique (Utilities|Array|MakeArray (Variables|Default|GetHISM)) _output_get)
      (Components|StaticMesh|SetStaticMesh _output_get (Variables|/Script/Engine.StaticMeshComponent|GetStaticMesh (LocalVariables|GetArray%20Element)))
      (Components|InstancedStaticMesh|AddInstance (LocalVariables|GetHISM%20Ref) (Transformation|GetWorldTransform (LocalVariables|GetArray%20Element)) true)
      (Rendering|Material|SetMaterial (LocalVariables|GetHISM%20Ref) 0 (Variables|Default|GetMaterial)))
    (for _array_element_2 _static_mesh_comp_array_2
      (Components|DestroyComponent _array_element_2))
    (Utilities|Array|Clear _static_mesh_comp_array_2)
    (return)))