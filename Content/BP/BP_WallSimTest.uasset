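; Test actor that builds a procedural, staggered stone wall with destroyed areas that collapse into physics-simulated rubble.
; The construction script places seeded, randomized stones as HISM instances.
; Stones inside Destructor spheres, or left unsupported according to downward box traces, become tagged simulating static mesh components.
; BeginPlay repositions these loose stones with random Y offsets, then after a delay Platon bakes their settled transforms into HISMs and destroys the components.
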(event EventBeginPlay
  (bind _index_sphere_collision_array (Variables|Default|GetIndex%20Sphere%20Collision_Array))
  (bind _l_size_y (Variables|Default|GetL%20Size%20Y))
  (for (_array_element _array_index) (Variables|Default|GetStatic%20Mesh%20Comp%20Array)
    (Transformation|SetRelativeTransform _array_element (Math|Transform|MakeTransform (+ (+ (Math|Vector|RotateVector (Utilities|Array|Get(acopy) (Variables|Default|GetStatic%20Mesh%20Location%20Array) _array_index) (Transformation|GetActorRotation)) (Transformation|GetActorLocation)) (Math|Vector|MakeVector 0.0 (Math|Random|RandomFloatinRangefromStream (Variables|Default|GetStream) (- _l_size_y 5e+01) (+ _l_size_y 5e+01)) 0.0)) (Transformation|GetActorRotation) "1.000000,1.000000,1.000000") false false))
  (Utilities|Array|Clear (Variables|Default|GetDestructor%20))
  (Utilities|FlowControl|Delay 5.0)
  (CallFunction|Platon)
  (for _array_element_2 _index_sphere_collision_array
    (Components|DestroyComponent _array_element_2)
    (Development|PrintText "Done" true true "(R=0.089121,G=1.000000,B=0.002958,A=1.000000)"))
  (Utilities|Array|Clear _index_sphere_collision_array))

(fn ConstructionScript
  (bind _stream (Variables|Default|GetStream))
  (bind _stream_2 (Variables|Default|GetStream))
  (bind _static_mesh_comp_array (Variables|Default|GetStatic%20Mesh%20Comp%20Array))
  (bind _hism_array_ref (Variables|Default|GetHISM%20Array%20Ref))
  (bind _index_sphere_collision_array (Variables|Default|GetIndex%20Sphere%20Collision_Array))
  (bind _stream_3 (Variables|Default|GetStream))
  (bind _outitem (Utilities|Array|Random _hism_array_ref))
  (bind _returnvalue (Math|Random|RandomIntegerinRangefromStream _stream 0 1))
  (bind _returnvalue_2 (Math|Random|RandomFloatinRangefromStream _stream_2 -5.0 5.0))
  (bind _returnvalue_3 (Math|Random|RandomFloatinRangefromStream _stream_3 0.7 1.0))
  (bind _returnvalue_4 (Math|Rotator|MakeRotator 0.0 0.0 _returnvalue_2))
  (bind _returnvalue_5 (* _returnvalue 180))
  (bind _returnvalue_6 (Math|Conversions|ToFloat(Integer) _returnvalue_5))
  (bind _returnvalue_7 (Math|Rotator|MakeRotator 0.0 0.0 _returnvalue_6))
  (bind _returnvalue_8 (Math|Rotator|CombineRotators _returnvalue_7 _returnvalue_4))
  (Utilities|Array|Clear (Variables|Default|GetStatic%20Mesh%20Location%20Array))
  (for _array_element _index_sphere_collision_array
    (Components|DestroyComponent _array_element))
  (Utilities|Array|Clear _index_sphere_collision_array)
  (for _array_element_2 _static_mesh_comp_array
    (Components|DestroyComponent _array_element_2))
  (Utilities|Array|Clear _static_mesh_comp_array)
  ;[0.439 0.8591 1] Set Static Mesh Array
  (for _array_element_3 (Variables|Default|GetStatic%20Mesh%20Array)
    (bind _output_get (Variables|Default|SetMesh%20Ref _array_element_3))
    (bind _returnvalue_9 (AddComponent|AddHierarchicalInstancedStaticMeshComponent false))
    (bind _output_get_2 (Variables|Default|SetHISM%20Ref _returnvalue_9))
    (Utilities|Array|AddUnique (Variables|Default|GetHISM%20Array%20Ref) _output_get_2)
    (Components|StaticMesh|SetStaticMesh _output_get_2 _output_get)
    (Variables|Default|SetStruct%20Mesh%20Data (Utilities|Struct|MakeStruct_Mesh_Data _output_get (Variables|Default|GetWall%20Material))))
  (if (and (> (Variables|Default|GetStone%20Z) 0) (> (Variables|Default|GetStone%20Y) 0))
    ;[0.1134 1 0] Get Mesh Size
    (Variables|Default|SetL%20Size%20X (.x (- (.max (StaticMesh|GetBoundingBox (Variables|Default|GetMesh%20Ref))) (.min (StaticMesh|GetBoundingBox (Variables|Default|GetMesh%20Ref))))))
    (Variables|Default|SetL%20Size%20Y (.y (- (.max (StaticMesh|GetBoundingBox (Variables|Default|GetMesh%20Ref))) (.min (StaticMesh|GetBoundingBox (Variables|Default|GetMesh%20Ref))))))
    (Variables|Default|SetL%20Size%20Z (.z (- (.max (StaticMesh|GetBoundingBox (Variables|Default|GetMesh%20Ref))) (.min (StaticMesh|GetBoundingBox (Variables|Default|GetMesh%20Ref))))))
    ;[1 0.7583 0] Set ZLocation
    (for _index (range 0 (- (Variables|Default|GetStone%20Z) 1))
      (bind _output_get_3 (Variables|Default|SetZ%20Index _index))
      (Variables|Default|SetL%20Stone%20ZLocation (+ (* _output_get_3 (Math|Vector|MakeVector 0.0 0.0 (Variables|Default|GetL%20Size%20Z))) (Math|Vector|MakeVector 0.0 0.0 (/ (Variables|Default|GetL%20Size%20Z) 2.0))))
      ;[1 0.777 0] Set XLocation
      (for _index_2 (range 0 (- (Variables|Default|GetStone%20Y) 1))
        (bind _output_get_4 (Variables|Default|SetY%20Index _index_2))
        (Variables|Default|SetL%20Stone%20XLocation (+ (* _output_get_4 (Math|Vector|MakeVector (Variables|Default|GetL%20Size%20X) 0.0 0.0)) (Math|Vector|MakeVector (/ (Variables|Default|GetL%20Size%20X) 2.0) 0.0 0.0)))
        (if (Utilities|Array|IsValidIndex (Variables|Default|GetDestructor%20))
          ;[0.01104 0.02123 0.349] Set Sphere Collision to Struct Pos
          (for _array_element_4 (Variables|Default|GetDestructor%20)
            (bind _returnvalue_10 (AddComponent|AddSphereComponent false (Math|Transform|MakeTransform (.Location (Utilities|Struct|BreakStruct_Destroyer _array_element_4)) "0, 0, 0" "1.000000,1.000000,1.000000")))
            (bind _output_get_5 (Variables|Default|SetIndex%20Sphere%20Collision _returnvalue_10))
            (Components|Sphere|SetSphereRadius _output_get_5 (.Radius (Utilities|Struct|BreakStruct_Destroyer _array_element_4)) true)
            (Utilities|Array|Add (Variables|Default|GetIndex%20Sphere%20Collision_Array) (Variables|Default|GetIndex%20Sphere%20Collision)))
          ;[1 0 0] Get Pos inter or outer Radius Destroyer
          (bind _array_element_5 (Utilities|Array|ForEachLoopwithBreak (Variables|Default|GetDestructor%20) :!label _label)
            (:LoopBody
              (if (>= (+ (Math|Float|Square (- (.X (Math|Vector|BreakVector (.Location (Utilities|Struct|BreakStruct_Destroyer _array_element_5)))) (.x (Variables|Default|GetL%20Stone%20XLocation)))) (Math|Float|Square (- (.Y (Math|Vector|BreakVector (.Location (Utilities|Struct|BreakStruct_Destroyer _array_element_5)))) 0.0)) (Math|Float|Square (- (.Z (Math|Vector|BreakVector (.Location (Utilities|Struct|BreakStruct_Destroyer _array_element_5)))) (.z (Variables|Default|GetL%20Stone%20ZLocation))))) (Math|Float|Square (.Radius (Utilities|Struct|BreakStruct_Destroyer _array_element_5))))
                (Variables|Default|SetInstantie%20? true)
                (else
                  (Variables|Default|SetInstantie%20? false)
                  (goto _label Break))))
            (:Completed
              (if (Variables|Default|GetInstantie%20?)
                (Utilities|FlowControl|ForLoopwithBreak 0 (- (Variables|Default|GetInstance%20Index) 1) :!label _label_2
                  (:LoopBody
                    ;[0.1461 1 0] Box Trace for Physique logique
                    (bind (_outhit _returnvalue_11) (Collision|BoxTraceByChannel (+ (Math|Vector|RotateVector (select (== (Math|Integer|%(Integer) (Variables|Default|GetZ%20Index) 2) 0) (+ (+ (Variables|Default|GetL%20Stone%20ZLocation) (Variables|Default|GetL%20Stone%20XLocation)) (Math|Vector|MakeVector (/ (Variables|Default|GetL%20Size%20X) 2.0) 0.0 0.0)) (+ (Variables|Default|GetL%20Stone%20ZLocation) (Variables|Default|GetL%20Stone%20XLocation))) (Transformation|GetActorRotation)) (Transformation|GetActorLocation)) (- (+ (Math|Vector|RotateVector (select (== (Math|Integer|%(Integer) (Variables|Default|GetZ%20Index) 2) 0) (+ (+ (Variables|Default|GetL%20Stone%20ZLocation) (Variables|Default|GetL%20Stone%20XLocation)) (Math|Vector|MakeVector (/ (Variables|Default|GetL%20Size%20X) 2.0) 0.0 0.0)) (+ (Variables|Default|GetL%20Stone%20ZLocation) (Variables|Default|GetL%20Stone%20XLocation))) (Transformation|GetActorRotation)) (Transformation|GetActorLocation)) (Math|Vector|MakeVector 0.0 0.0 (Variables|Default|GetL%20Size%20Z))) "20.000000,10.000000,10.000000" (Transformation|GetActorRotation) "TraceTypeQuery1" false 0 "None" false "(R=1.000000,G=0.000000,B=0.000000,A=1.000000)" "(R=0.000000,G=1.000000,B=0.000000,A=1.000000)" 1.0))
                    (if _returnvalue_11
                      (if (not (Components|ComponentHasTag (.HitComponent (Collision|BreakHitResult _outhit)) (Variables|Default|GetTag_Sim_Component)))
                        (Variables|Default|SetIs%20SM? false)
                        (goto _label_2 Break)
                        (else
                          _)))
                    (Variables|Default|SetIs%20SM? true))
                  (:Completed
                    (if (Variables|Default|GetIs%20SM?)
                      (Utilities|Array|Add (Variables|Default|GetStatic%20Mesh%20Location%20Array) (select (== (Math|Integer|%(Integer) (Variables|Default|GetZ%20Index) 2) 0) (+ (+ (Variables|Default|GetL%20Stone%20ZLocation) (Variables|Default|GetL%20Stone%20XLocation)) (Math|Vector|MakeVector (/ (Variables|Default|GetL%20Size%20X) 2.0) 0.0 0.0)) (+ (Variables|Default|GetL%20Stone%20ZLocation) (Variables|Default|GetL%20Stone%20XLocation))) :!label _label_3)
                      ;[1 1 1] Set Static Mesh for Physique
                      (bind _returnvalue_12 (AddComponent|AddStaticMeshComponent false (Math|Transform|MakeTransform (select (== (Math|Integer|%(Integer) (Variables|Default|GetZ%20Index) 2) 0) (+ (+ (Variables|Default|GetL%20Stone%20ZLocation) (Variables|Default|GetL%20Stone%20XLocation)) (Math|Vector|MakeVector (/ (Variables|Default|GetL%20Size%20X) 2.0) 0.0 0.0)) (+ (Variables|Default|GetL%20Stone%20ZLocation) (Variables|Default|GetL%20Stone%20XLocation))) _returnvalue_8 (Math|Vector|MakeVector 1.0 _returnvalue_3 1.0))))
                      (Utilities|Array|Add (Variables|Default|GetStatic%20Mesh%20Comp%20Array) _returnvalue_12)
                      (Components|StaticMesh|SetStaticMesh _returnvalue_12 (.OutItem (Utilities|Array|Random (Variables|Default|GetStatic%20Mesh%20Array))))
                      (Rendering|Material|SetMaterial _returnvalue_12 0 (Variables|Default|GetDestructed%20Material))
                      (Utilities|Array|AddUnique (Variables|/Script/Engine.ActorComponent|GetComponentTags _returnvalue_12) (Variables|Default|GetTag_Sim_Component))
                      (Physics|SetSimulatePhysics _returnvalue_12 true)
                      (else
                        ;[1 1 1] Add Instance
                        (bind _returnvalue_13 (Components|InstancedStaticMesh|AddInstance _outitem (Math|Transform|MakeTransform (select (== (Math|Integer|%(Integer) (Variables|Default|GetZ%20Index) 2) 0) (+ (+ (Variables|Default|GetL%20Stone%20ZLocation) (Variables|Default|GetL%20Stone%20XLocation)) (Math|Vector|MakeVector (/ (Variables|Default|GetL%20Size%20X) 2.0) 0.0 0.0)) (+ (Variables|Default|GetL%20Stone%20ZLocation) (Variables|Default|GetL%20Stone%20XLocation))) _returnvalue_8 (Math|Vector|MakeVector 1.0 _returnvalue_3 1.0)) false :!label _label_4))
                        (Variables|Default|SetInstance%20Index _returnvalue_13)
                        (Rendering|Material|SetMaterial _outitem 0 (Variables|Default|GetWall%20Material))
                        (Variables|Default|SetStruct%20Mesh%20Data (Utilities|Struct|MakeStruct_Mesh_Data 0 (Variables|Default|GetWall%20Material)))))))
                (else
                  (goto _label_3)))))
          (else
            (goto _label_4)))))))

(fn Platon
  (bind _static_mesh_comp_array (Variables|Default|GetStatic%20Mesh%20Comp%20Array))
  (bind _static_mesh_comp_array_2 (Variables|Default|GetStatic%20Mesh%20Comp%20Array))
  (if (Utilities|Array|IsValidIndex _static_mesh_comp_array)
    (for _array_element _static_mesh_comp_array
      (LocalVariables|SetArray%20Element _array_element)
      (Rendering|SetVisibility (LocalVariables|GetArray%20Element) false false)
      (bind _returnvalue (AddComponent|AddHierarchicalInstancedStaticMeshComponent false))
      (bind _output_get (Variables|Default|SetHISM%20Ref _returnvalue))
      (Utilities|Array|AddUnique (Variables|Default|GetHISM%20Array%20Ref) _output_get)
      (Components|StaticMesh|SetStaticMesh _output_get (Variables|/Script/Engine.StaticMeshComponent|GetStaticMesh (LocalVariables|GetArray%20Element)))
      (Components|InstancedStaticMesh|AddInstance (Variables|Default|GetHISM%20Ref) (Transformation|GetWorldTransform (LocalVariables|GetArray%20Element)) true)
      (Rendering|Material|SetMaterial (Variables|Default|GetHISM%20Ref) 0 (Utilities|Struct|BreakStruct_Mesh_Data (Variables|Default|GetStruct%20Mesh%20Data))))
    (for _array_element_2 _static_mesh_comp_array_2
      (Components|DestroyComponent _array_element_2))
    (Utilities|Array|Clear _static_mesh_comp_array_2)
    (return)))