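; Construction-script actor that randomly scatters static meshes around a list of configurable zones.
; Each Structure entry builds a circular spline from computed points and tangents to outline its location and radius.
; Every listed mesh gets HISM components, picked at random per instance from an accumulating array.
; Seeded-stream offsets and yaw place instances within a square spanning the radius, not clipped to the circle, at the zone's height and scale.
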(event EventBeginPlay)

(event Collision|EventActorBeginOverlap
  (params (OtherActor :type Actor%20Object%20Reference)))

(event EventTick
  (params (DeltaSeconds :type Float%20%28single-precision%29)))

(fn ConstructionScript
  (Components|InstancedStaticMesh|ClearInstances (Variables|Default|GetHISM%20Ref))
  ;[0.15 0.15 0.15 0.5] Set Struct Data
  (for (_array_element _array_index) (Variables|Default|GetStructure)
    (Variables|Default|SetNb_Struct_Index _array_index)
    (Variables|Default|SetZone%20Location (.Location (Utilities|Struct|BreakSt_LocRandomMesh _array_element)))
    (Variables|Default|SetL_Radius (.Radius (Utilities|Struct|BreakSt_LocRandomMesh _array_element)))
    (Variables|Default|SetNb%20Static%20Mesh (.NbStaticMesh (Utilities|Struct|BreakSt_LocRandomMesh _array_element)))
    (Variables|Default|SetScale (.Scale (Utilities|Struct|BreakSt_LocRandomMesh _array_element)))
    (bind _returnvalue (AddComponent|AddSplineComponent false))
    (Variables|Default|SetL%20Spline%20Component _returnvalue)
    (Spline|ClearSplinePoints (Variables|Default|GetL%20Spline%20Component) true)
    (if (Utilities|Array|IsValidIndex (Variables|Default|GetStructure))
      ;[0.15 0.15 0.15 0.5] Tangent Math
      (for _index (range 0 (- (Variables|Default|GetL_SplinePoints) 1))
        (Variables|Default|SetL_Index%20Point _index)
        (Variables|Default|SetL_SplinePoint (Math|Vector|MakeVector (+ (* (Math|Trig|Sin(Degrees) (Math|Float|MapRangeClamped (Math|Conversions|ToFloat(Integer) (Variables|Default|GetL_Index%20Point)) 0.0 (Math|Conversions|ToFloat(Integer) (- (Variables|Default|GetL_SplinePoints) 1)) 0.0 (Math|Conversions|ToFloat(Integer) (|(360-(360/Segments)) (Variables|Default|GetL_SplinePoints))))) (Variables|Default|GetL_Radius)) (.x (Variables|Default|GetZone%20Location))) (+ (* (Math|Trig|Cos(Degrees) (Math|Float|MapRangeClamped (Math|Conversions|ToFloat(Integer) (Variables|Default|GetL_Index%20Point)) 0.0 (Math|Conversions|ToFloat(Integer) (- (Variables|Default|GetL_SplinePoints) 1)) 0.0 (Math|Conversions|ToFloat(Integer) (|(360-(360/Segments)) (Variables|Default|GetL_SplinePoints))))) (Variables|Default|GetL_Radius)) (.y (Variables|Default|GetZone%20Location))) (.z (Variables|Default|GetZone%20Location))))
        (Spline|AddSplinePoint (Variables|Default|GetL%20Spline%20Component) (Variables|Default|GetL_SplinePoint) "Local" true)
        (Variables|Default|SetL_Rotation (Math|Rotator|FindLookatRotation (Variables|Default|GetL_SplinePoint) (Variables|Default|GetZone%20Location)))
        (Variables|Default|SetL_TangentAtSplinePoint (* (Math|Vector|GetRightVector (Variables|Default|GetL_Rotation)) (* (Variables|Default|GetL_Radius) (|(4*(tan(((D2R((360/Segments)))/4)))) (Variables|Default|GetL_SplinePoints)))))
        (Spline|SetTangentatSplinePoint (Variables|Default|GetL%20Spline%20Component) (Variables|Default|GetL_Index%20Point) (Variables|Default|GetL_TangentAtSplinePoint) "Local" true))
      ;[0.15 0.15 0.15 0.5] Set Static Mesh
      (for _array_element_2 (Variables|Default|GetStatic%20Mesh%20Index)
        (bind _output_get (Variables|Default|SetMesh%20Ref _array_element_2))
        (bind _returnvalue_2 (AddComponent|AddHierarchicalInstancedStaticMeshComponent false))
        (bind _output_get_2 (Variables|Default|SetHISM%20Ref _returnvalue_2))
        (Utilities|Array|AddUnique (Variables|Default|GetHISM%20Array%20Ref) _output_get_2)
        (Components|StaticMesh|SetStaticMesh _output_get_2 _output_get))
      ;[0.15 0.15 0.15 0.5] Set Instance
      (for _index_2 (range 0 (- (Variables|Default|GetNb%20Static%20Mesh) 1))
        (Components|InstancedStaticMesh|AddInstance (.OutItem (Utilities|Array|Random (Variables|Default|GetHISM%20Array%20Ref))) (Math|Transform|MakeTransform (Math|Vector|MakeVector (+ (.x (Variables|Default|GetZone%20Location)) (Math|Random|RandomFloatinRangefromStream (Variables|Default|GetStream) (* (Variables|Default|GetL_Radius) -1.0) (Variables|Default|GetL_Radius))) (+ (.y (Variables|Default|GetZone%20Location)) (Math|Random|RandomFloatinRangefromStream (Variables|Default|GetStream) (* (Variables|Default|GetL_Radius) -1.0) (Variables|Default|GetL_Radius))) (.z (Variables|Default|GetZone%20Location))) (Math|Rotator|MakeRotator 0.0 0.0 (Math|Random|RandomFloatinRangefromStream (Variables|Default|GetStream) 0.0 3.6e+02)) (Math|Conversions|ToVector(Float) (Variables|Default|GetScale))) false)))))